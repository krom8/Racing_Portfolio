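; Learning Agents interactor that defines what the AI running pawn (BP_AIRunningPawn) senses and controls for driving.
; Each agent refreshes its data, then feeds five arrow results in as float observations.
; Two float actions drive the pawn: throttle/brake is clamped to forward-only input, while steering passes straight through to the turn value.
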(event `self.SetupObservations`
  (bind _returnvalue (`FloatObservation.AddFloatObservation` null "Arrow1Observation"))
  (set `self.Arrow1Observation` _returnvalue)
  (bind _returnvalue_2 (`FloatObservation.AddFloatObservation` null "Arrow2Observation"))
  (set `self.Arrow2Observation` _returnvalue_2)
  (bind _returnvalue_3 (`FloatObservation.AddFloatObservation` null "Arrow3Observation"))
  (set `self.Arrow3Observation` _returnvalue_3)
  (bind _returnvalue_4 (`FloatObservation.AddFloatObservation` null "Arrow4Observation"))
  (set `self.Arrow4Observation` _returnvalue_4)
  (bind _returnvalue_5 (`FloatObservation.AddFloatObservation` null "Arrow5Observation"))
  (set `self.Arrow5Observation` _returnvalue_5))

(event `self.SetObservations`
  (params (AgentIds :type "Array of Integer (by ref)"))
  (for _array_element AgentIds
    (bind _returnvalue (`self.GetAgent` _array_element "/Game/BP_AIRunning/BP_AIRunningPawn.BP_AIRunningPawn_C"))
    (`/Game/BP_AIRunning/BP_AIRunningPawn.GetData` _returnvalue)
    (`FloatObservation.SetFloatObservation` (`self.Arrow1Observation`) _array_element (`/Game/BP_AIRunning/BP_AIRunningPawn.ArrowResult1` _returnvalue))
    (`FloatObservation.SetFloatObservation` (`self.Arrow2Observation`) _array_element (`/Game/BP_AIRunning/BP_AIRunningPawn.ArrowResult2` _returnvalue))
    (`FloatObservation.SetFloatObservation` (`self.Arrow3Observation`) _array_element (`/Game/BP_AIRunning/BP_AIRunningPawn.ArrowResult3` _returnvalue))
    (`FloatObservation.SetFloatObservation` (`self.Arrow4Observation`) _array_element (`/Game/BP_AIRunning/BP_AIRunningPawn.ArrowResult4` _returnvalue))
    (`FloatObservation.SetFloatObservation` (`self.Arrow5Observation`) _array_element (`/Game/BP_AIRunning/BP_AIRunningPawn.ArrowResult5` _returnvalue))))

(event `self.SetupActions`
  (`|ExecutionSequence`
    (:`then_0`
      (bind _returnvalue (`FloatAction.AddFloatAction` null "ThrottleBrakeAction" 2.0))
      (set `self.ThrottleBrakeAction` _returnvalue))
    (:`then_1`
      (bind _returnvalue_2 (`FloatAction.AddFloatAction` null "SteeringAction" 2.0))
      (set `self.SteeringAction` _returnvalue_2))))

(event `self.GetActions`
  (params (AgentIds :type "Array of Integer (by ref)"))
  (for _array_element AgentIds
    (`|ExecutionSequence`
      (:`then_0`
        (bind _returnvalue (`FloatAction.GetFloatAction` (`self.ThrottleBrakeAction`) _array_element))
        (bind _returnvalue_2 (`self.GetAgent` _array_element "/Game/BP_AIRunning/BP_AIRunningPawn.BP_AIRunningPawn_C"))
        (set `AIRunningPawn.ForwardFloat` (`KismetMathLibrary.FClamp` _returnvalue) _returnvalue_2))
      (:`then_1`
        (bind _returnvalue_3 (`FloatAction.GetFloatAction` (`self.SteeringAction`) _array_element))
        (set `AIRunningPawn.TurnFloat` _returnvalue_3 _returnvalue_2)))))