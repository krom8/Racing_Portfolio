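; BP_StyleTransferManager is an actor that switches on real-time style transfer rendering from the keyboard.
; It enables player input on BeginPlay; pressing 1 calls SetStyle, turns on the RealtimeStyleTransfer console variable and sets a Check flag.
; While Check is set, Tick reissues the enable command every frame and prints a debug string; nothing in the graph clears it.
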(event `Key|One`
  (params (Key :type "Key Structure"))
  (:`Pressed`
    (`STBlueprintLibrary.SetStyle`)
    (`KismetSystemLibrary.ExecuteConsoleCommand` "r.RealtimeStyleTransfer.Enable 1" null)
    (set `self.check` true)))

(event `self.ReceiveBeginPlay`
  (`self.EnableInput` (`GameplayStatics.GetPlayerController` 0)))

(event `self.ReceiveTick`
  (params (DeltaSeconds :type "Float (single-precision)"))
  (if (`self.check`)
    (`KismetSystemLibrary.ExecuteConsoleCommand` "r.RealtimeStyleTransfer.Enable 1" null)
    (`KismetSystemLibrary.PrintString` "tickticktick")))

(fn `UserConstructionScript`)