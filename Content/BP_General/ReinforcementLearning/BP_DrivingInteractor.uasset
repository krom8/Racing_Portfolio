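; Learning Agents interactor that defines what AI driving agents (BP_AIRunningPawn) observe and control on a spline track.
; Observations use a spline helper on BP_TrackSpline: track position and direction relative to the car, lap progress as an angle, planar velocity, and distance from the spline.
; Two float actions set steering and clamped throttle, with brake input always zero.
; An older arrow-ratio observation setup remains as unconnected nodes.
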(event `self.SetupObservations`
  (`|ExecutionSequence`
    (:`then_0`
      (bind _returnvalue (`PlanarPositionObservation.AddPlanarPositionObservation` null "TrackPositionObservation"))
      (set `self.TrackPositionObservation` _returnvalue)
      (bind _returnvalue_2 (`PlanarDirectionObservation.AddPlanarDirectionObservation` null "TrackDirectionObservation"))
      (set `self.TrackDirectionObservation` _returnvalue_2))
    (:`then_1`
      (bind _returnvalue_3 (`AngleObservation.AddAngleObservation` null "TrackGlobalPositionObservation"))
      (set `self.TrackGlobalPositionObservation` _returnvalue_3)
      (bind _returnvalue_4 (`PlanarVelocityObservation.AddPlanarVelocityObservation` null "CarVelocityObservation"))
      (set `self.CarVelocityObservation` _returnvalue_4))
    (:`then_2`
      (bind _returnvalue_5 (`SplineComponentHelper.AddSplineComponentHelper` null "SplineComponentHelper"))
      (bind _output_get (set `self.SplineComponentHelper` _returnvalue_5))
      (`/Engine/EditorBlueprintResources/StandardMacros.IsValid` _output_get
        (:`Is Valid`
          (bind _returnvalue_6 (`GameplayStatics.GetActorOfClass` "/Game/BP_General/ReinforcementLearning/BP_TrackSpline.BP_TrackSpline_C"))
          (set `self.TrackSpline` (`/Game/BP_General/ReinforcementLearning/BP_TrackSpline.Spline` _returnvalue_6)))
        (:`Is Not Valid`
          (`KismetSystemLibrary.PrintString` "Hello" true true (struct :`R` 1.0 :`A` 1.0) 40.0))))
    (:`then_3`
      (bind _returnvalue_7 (`FloatObservation.AddFloatObservation` null "Distance" 1000.0))
      (set `self.DistanceObs` _returnvalue_7))))

(event `self.SetObservations`
  (params (AgentIds :type "Array of Integer (by ref)"))
  (for _array_element AgentIds
    (bind _returnvalue (`self.GetAgent` _array_element "/Game/BP_AIRunning/BP_AIRunningPawn.BP_AIRunningPawn_C"))
    (bind _returnvalue_2 (`Actor.K2_GetActorLocation` _returnvalue))
    (bind _returnvalue_3 (`SplineComponentHelper.GetDistanceAlongSplineAtPosition` (`self.SplineComponentHelper`) _array_element (`self.TrackSpline`) _returnvalue_2 "World"))
    (`|ExecutionSequence`
      (:`then_0`
        (bind _returnvalue_4 (`SplineComponentHelper.GetPositionAtDistanceAlongSpline` (`self.SplineComponentHelper`) _array_element (`self.TrackSpline`) _returnvalue_3 "World"))
        (bind _returnvalue_5 (`Actor.K2_GetActorRotation` _returnvalue))
        (`PlanarPositionObservation.SetPlanarPositionObservation` (`self.TrackPositionObservation`) _array_element _returnvalue_4 _returnvalue_2 _returnvalue_5))
      (:`then_1`
        (bind _returnvalue_6 (`SplineComponentHelper.GetDirectionAtDistanceAlongSpline` (`self.SplineComponentHelper`) _array_element (`self.TrackSpline`) _returnvalue_3 "World"))
        (`PlanarDirectionObservation.SetPlanarDirectionObservation` (`self.TrackDirectionObservation`) _array_element _returnvalue_6 _returnvalue_5))
      (:`then_2`
        (bind _returnvalue_7 (`SplineComponentHelper.GetProportionAlongSplineAsAngle` (`self.SplineComponentHelper`) _array_element (`self.TrackSpline`) _returnvalue_3))
        (`AngleObservation.SetAngleObservation` (`self.TrackGlobalPositionObservation`) _array_element _returnvalue_7 0.0))
      (:`then_3`
        (`PlanarVelocityObservation.SetPlanarVelocityObservation` (`self.CarVelocityObservation`) _array_element (`Actor.GetVelocity` _returnvalue) _returnvalue_5))
      (:`then_4`
        (bind _returnvalue_8 (`Actor.K2_GetActorLocation` _returnvalue))
        (bind _returnvalue_9 (`SplineComponentHelper.GetNearestPositionOnSpline` (`self.SplineComponentHelper`) _array_element (`self.TrackSpline`) _returnvalue_8 "World"))
        (`FloatObservation.SetFloatObservation` (`self.DistanceObs`) _array_element (`KismetMathLibrary.Vector_Distance` _returnvalue_8 _returnvalue_9))))))

(event `self.SetupActions`
  (`|ExecutionSequence`
    (:`then_0`
      (bind _returnvalue (`FloatAction.AddFloatAction` null "ThrottleBrakeAction" 2.0))
      (set `self.ThrottleBrakeAction` _returnvalue))
    (:`then_1`
      (bind _returnvalue_2 (`FloatAction.AddFloatAction` null "SteeringAction" 2.0))
      (set `self.SteeringAction` _returnvalue_2))))

(event `self.GetActions`
  (params (AgentIds :type "Array of Integer (by ref)"))
  (for _array_element AgentIds
    (`|ExecutionSequence`
      (:`then_0`
        (bind _returnvalue (`FloatAction.GetFloatAction` (`self.ThrottleBrakeAction`) _array_element))
        (bind _returnvalue_2 (`self.GetAgent` _array_element "/Game/BP_AIRunning/BP_AIRunningPawn.BP_AIRunningPawn_C"))
        (bind _vehiclemovementcomponent (`WheeledVehiclePawn.VehicleMovementComponent` _returnvalue_2))
        (`ChaosVehicleMovementComponent.SetThrottleInput` _vehiclemovementcomponent (`KismetMathLibrary.FClamp` _returnvalue))
        (`ChaosVehicleMovementComponent.SetBrakeInput` _vehiclemovementcomponent 0.0))
      (:`then_1`
        (bind _returnvalue_3 (`FloatAction.GetFloatAction` (`self.SteeringAction`) _array_element))
        (`ChaosVehicleMovementComponent.SetSteeringInput` (`WheeledVehiclePawn.VehicleMovementComponent` _returnvalue_2) _returnvalue_3)))))